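; Blueprint for the Battery Collector character that shows its current power level through body color.
; The construction script creates a dynamic material instance from the mesh's first material and stores it as PowerMaterial.
; The PowerChangeEffect event sets that material's BodyColor, blending from blue when empty to orange at or above initial power, using the clamped current-to-initial power ratio.
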(event EventBeginPlay)

(event Collision|EventActorBeginOverlap
  (params (OtherActor :type Actor%20Object%20Reference)))

(event EventTick
  (params (DeltaSeconds :type Float%20%28single-precision%29)))

(event EventPowerChangeEffect
  (Rendering|Material|SetVectorParameterValue (Variables|Default|GetPowerMaterial) "BodyColor" (Math|Color|Lerp(LinearColor) "(R=0.000000,G=0.533035,B=1.000000,A=1.000000)" "(R=1.000000,G=0.339220,B=0.000000,A=1.000000)" (Math|Float|Clamp(Float) (/ (Class|BatteryCollectorCharacter|GetCurrentPower) (Class|BatteryCollectorCharacter|GetInitialPower)))) :!class /Script/Engine.MaterialInstanceDynamic))

(fn ConstructionScript
  (bind _mesh (Variables|Character|GetMesh))
  (bind _returnvalue (Rendering|Material|CreateDynamicMaterialInstance _mesh 0 (Utilities|Array|Get(acopy) (Rendering|Material|GetMaterials _mesh)) "None" :!class /Script/Engine.PrimitiveComponent))
  (Variables|Default|SetPowerMaterial _returnvalue))